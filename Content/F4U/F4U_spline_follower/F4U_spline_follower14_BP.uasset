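; Spline follower Blueprint that flies an F4U Corsair along a preset path with engine audio.
; On BeginPlay it waits a long fixed delay, then attaches a Messerschmitt Bf109 engine sound to the Corsair and plays a timeline.
; The timeline's TravelDistance, scaled by spline length, sets the plane's world location and its relative rotation from the spline's local-space rotation each update.
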(event EventBeginPlay
  (bind _spline (Variables|Default|GetSpline))
  (Utilities|FlowControl|Delay 125.0)
  (Audio|SpawnSoundAttached "/Game/StarterContent/Audio/Messerschmitt_Bf-109_3.Messerschmitt_Bf-109_3" (Variables|Default|Getcorsair) "None" "0, 0, 0" "0, 0, 0" "KeepRelativeOffset" false 1.0 1.0 0.0 "/Game/sound/plane_engine.plane_engine" 0)
  (bind _travel_distance (Timeline|Timeline_0 Play)
    (:Update
      (Transformation|SetWorldLocation (Variables|Default|Getcorsair) (Spline|GetLocationatDistanceAlongSpline _spline (* _travel_distance (Spline|GetSplineLength (Variables|Default|GetSpline))) "World") false false)
      (Transformation|SetRelativeRotation (Variables|Default|Getcorsair) (Spline|GetRotationatDistanceAlongSpline _spline (* _travel_distance (Spline|GetSplineLength (Variables|Default|GetSpline))) "Local") false false))))

(fn ConstructionScript)